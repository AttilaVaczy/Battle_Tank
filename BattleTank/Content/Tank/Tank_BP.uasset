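; Tank Blueprint that assembles the tank from separate body, turret, barrel and track components.
; The construction script attaches the turret and both tracks to the Tank component, and the barrel to the turret's Barrel socket, all keeping relative transforms.
; The event graph holds only disabled placeholder events, so the Blueprint's graphs add no runtime behavior.
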(event EventBeginPlay)

(event Collision|EventActorBeginOverlap
  (params (OtherActor :type Actor%20Object%20Reference)))

(event EventTick
  (params (DeltaSeconds :type Float%20%28single-precision%29)))

(fn ConstructionScript
  (Transformation|AttachComponentToComponent (Variables|Default|GetTurret) (Variables|Default|GetTank) "None" "KeepRelative" "KeepRelative" "KeepRelative" true)
  (Transformation|AttachComponentToComponent (Variables|Default|GetBarrel) (Variables|Default|GetTurret) "Barrel" "KeepRelative" "KeepRelative" "KeepRelative" true)
  (Transformation|AttachComponentToComponent (Variables|Default|GetTrack_Left) (Variables|Default|GetTank) "None" "KeepRelative" "KeepRelative" "KeepRelative" true)
  (Transformation|AttachComponentToComponent (Variables|Default|GetTrack_Right) (Variables|Default|GetTank) "None" "KeepRelative" "KeepRelative" "KeepRelative" true))